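; BP_Enemy_Base is the base enemy Blueprint, handling a melee attack, death and access to a patrol route.
; Attack plays a sped-up sword slash montage and calls OnAttackEnd whether it completes or is interrupted.
; When NPCStats fires OnDeath, a valid controller unpossesses the enemy and a death montage plays.
; Just before that montage ends, it sets IsDead on the ABP_Manny anim instance, avoiding a blend out of the death pose.
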(event `Attack`
  (`|PlayMontage` (`self.Mesh`) "/Game/Animations/SwordAndShieldSlash_UE_Anim_Montage.SwordAndShieldSlash_UE_Anim_Montage" 2.0
    (:`OnCompleted`
      _)
    (:`OnInterrupted`
      _))
  (`self.OnAttackEnd`))

(event `self.NPCStats.OnDeath`
  (bind _returnvalue (`self.GetController`))
  (`/Engine/EditorBlueprintResources/StandardMacros.IsValid` _returnvalue
    (:`Is Valid`
      (`Controller.UnPossess` _returnvalue)
      (`|PlayMontage` (`self.Mesh`) (`self.DeathMontage to Play`)
        (:`then`
          (`KismetSystemLibrary.Delay` (- (`AnimationAsset.GetPlayLength` (`self.DeathMontage to Play`)) 0.01))
          (bind _asabp_manny (cast `/Game/Characters/Mannequins/Animations/ABP_Manny` (`SkeletalMeshComponent.GetAnimInstance` (`self.Mesh`))))
          (set `/Game/Characters/Mannequins/Animations/ABP_Manny.IsDead` true _asabp_manny))))))

(fn `GetPatrolRoute`
  (returns (PatrolRoute :type "/Game/AI/BP_PatrolPath Object Reference"))
  (return (`self.PatrolRoute`)))

(fn `UserConstructionScript`)